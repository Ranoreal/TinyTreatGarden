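; Player character Blueprint providing look, camera-yaw-relative movement and sprinting through Enhanced Input actions.
; Holding sprint sets IsRunning, which Tick reads to interpolate walk speed, with separate ramp-up and ramp-down rates, and camera FOV.
; Tick also starts an idle, walk or sprint legacy camera shake for head bob, based on velocity and IsRunning.
; Sprint and StopSprint functions set speed instantly but are not called in this graph.
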(event `self.ReceiveTick`
  (params (DeltaSeconds :type "Float (single-precision)"))
  ; Tick
  (`self.Sprinting`)
  (`self.HeadBob`)
  (`self.FovChange`))

(event `EnhancedInput|/Game/Project/Inputs/IA_Look`
  (params (ActionValue :type "Vector2D Structure") (ElapsedSeconds :type "Float (double-precision)") (TriggeredSeconds :type "Float (double-precision)") (InputAction :type "InputAction Object Reference" :default "/Game/Project/Inputs/IA_Look.IA_Look"))
  ; Movement
  (:`Triggered`
    (`self.AddControllerYawInput` ActionValue_X)
    (`self.AddControllerPitchInput` ActionValue_Y)))

(event `HeadBob`
  (bind _returnvalue (`GameplayStatics.GetPlayerCameraManager` 0))
  ; Head Bob
  (if (> (`KismetMathLibrary.VSize` (`self.GetVelocity`)) 0.0)
    (if (`self.IsRunning?`)
      (`LegacyCameraShake.StartLegacyCameraShake` _returnvalue "/Game/Project/Blueprints/Player/HeadBob/BP_Sprint.BP_Sprint_C" (`KismetMathLibrary.FInterpTo` 0.0 1.0 (`GameplayStatics.GetWorldDeltaSeconds`)))
      (else
        (`LegacyCameraShake.StartLegacyCameraShake` _returnvalue "/Game/Project/Blueprints/Player/HeadBob/BP_Walk.BP_Walk_C" (`KismetMathLibrary.FInterpTo` 0.0 1.0 (`GameplayStatics.GetWorldDeltaSeconds`)))))
    (else
      (`LegacyCameraShake.StartLegacyCameraShake` _returnvalue "/Game/Project/Blueprints/Player/HeadBob/BP_Idle.BP_Idle_C" (`KismetMathLibrary.FInterpTo` 0.0 1.0 (`GameplayStatics.GetWorldDeltaSeconds`))))))

(event `EnhancedInput|/Game/Project/Inputs/IA_MoveFoward`
  (params (ActionValue :type "Float (double-precision)") (ElapsedSeconds :type "Float (double-precision)") (TriggeredSeconds :type "Float (double-precision)") (InputAction :type "InputAction Object Reference" :default "/Game/Project/Inputs/IA_MoveFoward.IA_MoveFoward"))
  (bind (_returnvalue_roll _returnvalue_pitch _returnvalue_yaw) (`KismetMathLibrary.BreakRotator` (`self.GetControlRotation`)))
  ; Movement
  (:`Triggered`
    (`self.AddMovementInput` (`KismetMathLibrary.GetForwardVector` (`KismetMathLibrary.MakeRotator` 0.0 0.0 _returnvalue_yaw)) ActionValue)))

(event `EnhancedInput|/Game/Project/Inputs/IA_MoveRight`
  (params (ActionValue :type "Float (double-precision)") (ElapsedSeconds :type "Float (double-precision)") (TriggeredSeconds :type "Float (double-precision)") (InputAction :type "InputAction Object Reference" :default "/Game/Project/Inputs/IA_MoveRight.IA_MoveRight"))
  (bind (_returnvalue_roll _returnvalue_pitch _returnvalue_yaw) (`KismetMathLibrary.BreakRotator` (`self.GetControlRotation`)))
  ; Movement
  (:`Triggered`
    (`self.AddMovementInput` (`KismetMathLibrary.GetRightVector` (`KismetMathLibrary.MakeRotator` 0.0 0.0 _returnvalue_yaw)) ActionValue)))

(event `EnhancedInput|/Game/Project/Inputs/IA_Sprint`
  (params (ActionValue :type Boolean) (ElapsedSeconds :type "Float (double-precision)") (TriggeredSeconds :type "Float (double-precision)") (InputAction :type "InputAction Object Reference" :default "/Game/Project/Inputs/IA_Sprint.IA_Sprint"))
  ; Sprinting
  (:`Triggered`
    (set `self.IsRunning?` true))
  (:`Completed`
    (set `self.IsRunning?` false)))

(event `FovChange`
  ; Fov Change
  (if (`self.IsRunning?`)
    (set `self.TargetFOV` (`self.SprintFOV`))
    (bind _output_get (set `self.CurrentFOV` (`KismetMathLibrary.FInterpTo` (`self.CurrentFOV`) (`self.TargetFOV`) (`GameplayStatics.GetWorldDeltaSeconds`) 8.0)))
    (`CameraComponent.SetFieldOfView` (`self.Camera`) _output_get)
    (else
      (set `self.TargetFOV` (`self.DefaultFOV`))
      (bind _output_get_2 (set `self.CurrentFOV` (`KismetMathLibrary.FInterpTo` (`self.CurrentFOV`) (`self.TargetFOV`) (`GameplayStatics.GetWorldDeltaSeconds`) 8.0)))
      (`CameraComponent.SetFieldOfView` (`self.Camera`) _output_get_2))))

(event `Sprinting`
  ; Sprinting
  (if (`self.IsRunning?`)
    (set `CharacterMovementComponent.MaxWalkSpeed` (`KismetMathLibrary.FInterpTo` (`CharacterMovementComponent.MaxWalkSpeed` (`self.CharacterMovement`)) (`self.SprintSpeed`) (`GameplayStatics.GetWorldDeltaSeconds`) (`self.SpeedUpTime`)) (`self.CharacterMovement`))
    (else
      (set `CharacterMovementComponent.MaxWalkSpeed` (`KismetMathLibrary.FInterpTo` (`CharacterMovementComponent.MaxWalkSpeed` (`self.CharacterMovement`)) (`self.WalkSpeed`) (`GameplayStatics.GetWorldDeltaSeconds`) (`self.SpeedDownTime`)) (`self.CharacterMovement`)))))

(fn `Sprint`
  (set `CharacterMovementComponent.MaxWalkSpeed` (`self.SprintSpeed`) (`self.CharacterMovement`)))

(fn `StopSprint`
  (set `CharacterMovementComponent.MaxWalkSpeed` (`self.WalkSpeed`) (`self.CharacterMovement`)))

(fn `UserConstructionScript`)